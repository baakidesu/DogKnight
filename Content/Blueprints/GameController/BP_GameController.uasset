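; Game controller that runs timed enemy waves, kill-based player leveling and chest respawns.
; Tick counts seconds and starts waves from per-wave maps, spawning random enemies at recursively sampled reachable points around the player; all difficulties currently use EasyEnemies.
; Enemy deaths save the kill total and level up the player at a rising threshold.
; ChestDestroy spawns a chest at a ChestPossibleLocationds entry, though that array's target-point lookup is disconnected.
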(event EventChestDestroy
  (params (Actor :type Actor%20Object%20Reference))
  (CallFunction|CreateChest))

(event EventBeginPlay
  (bind _returnvalue (Actor|GetActorOfClass "/Game/Blueprints/Characters/Player/BP_Player.BP_Player_C"))
  (Variables|Player|SetPlayer _returnvalue)
  (bind _returnvalue_2 (SaveGame|CreateSaveGameObject "/Game/Blueprints/GameController/SaveGame.SaveGame_C"))
  (Variables|Default|SetSaveGame _returnvalue_2))

(event EventDieMessagetoSpawner
  (bind _result (Math|Integer|IncrementInt (Variables|Default|GetKilledEnemyCount))
    (:%20%20
      (Variables|Default|SetLevelEnemyCounter (Math|Conversions|ToFloat(Integer) _result))
      (CallFunction|Save (Variables|Default|GetSaveGame))
      (if (== (Variables|Default|GetLevelUp) (Variables|Default|GetLevelEnemyCounter))
        (Variables|Default|SetLevelEnemyCounter 0.0)
        (Variables|Default|SetLevelUp (+ (Variables|Default|GetLevelUp) 1e+01))
        (Class|BPIControllertoPlayer|IncreaseLevel(Message) (Variables|Player|GetPlayer)))
      (Default|CallDPEnemyCount (Variables|Default|GetLevelEnemyCounter)))))

(event EventTick
  (params (DeltaSeconds :type Float%20%28single-precision%29))
  (CallFunction|CountSeconds DeltaSeconds)
  (if (== (Variables|Time|GetCurrentTime) (.Value (Utilities|Map|Find (Variables|Wave|GetWaveTriggers) (Variables|Wave|GetCurrentWave))))
    (CallFunction|StartWave)))

(fn ConstructionScript)

(fn GetWaveHardnessandEnemyCount
  (params (Wave :type Integer%20%28by%20ref%29))
  (return (.Value (Utilities|Map|Find (Variables|Wave|GetWaveHardness) Wave)) (.Value (Utilities|Map|Find (Variables|Wave|GetWaveEnemyCount) Wave))))

(fn StartWave
  (bind _currentwave (Variables|Wave|GetCurrentWave))
  (bind _easyenemies (Variables|EnemyTypes|GetEasyEnemies))
  (bind (_hardness _enemycount) (CallFunction|GetWaveHardnessandEnemyCount _currentwave))
  (switch Utilities|FlowControl|Switch|SwitchonEnum_Hardness _hardness
    (:NewEnumerator0
      (CallFunction|SpawnEnemies _enemycount _easyenemies))
    (:NewEnumerator1
      (CallFunction|SpawnEnemies _enemycount _easyenemies))
    (:NewEnumerator2
      (CallFunction|SpawnEnemies _enemycount _easyenemies)))
  (Math|Integer|IncrementInt (Variables|Wave|GetCurrentWave)))

(fn SpawnEnemies
  (params (EnemyCount :type Integer) (Array :type Array%20of%20BP%20Enemy%20Class%20References))
  (bind _outitem (Utilities|Array|Random Array))
  (for _index (range 1 EnemyCount)
    (if (Utilities|IsValidClass _outitem)
      (bind _randomlocation (CallFunction|GetReachableTransform))
      (bind _returnvalue (Game|SpawnActorfromClass _outitem _randomlocation "AdjustIfPossibleButAlwaysSpawn" "MultiplyWithRoot" 0 0))
      (Utilities|IsValid _returnvalue
        (:Is%20Valid
          (Math|Integer|IncrementInt (Variables|Wave|GetActiveEnemyCount)
            (:%20%20
              (Variables|/Game/Blueprints/Characters/Enemies/BP_Enemy.BP_Enemy_C|SetBP_GameController _returnvalue self)))))
      (else
        (return))))
  (return))

(fn CountSeconds
  (params (DeltaTime :type Float%20%28double-precision%29))
  (bind _output_get (Variables|Time|SetAccumulatedTime (+ DeltaTime (Variables|Time|GetAccumulatedTime))))
  (if (>= _output_get 1.0)
    (Variables|Time|SetAccumulatedTime (- (Variables|Time|GetAccumulatedTime) 1.0))
    (Math|Integer|IncrementInt (Variables|Time|GetCurrentTime)
      (:%20%20
        (return)))))

(fn GetReachableTransform
  (bind _output_get (LocalVariables|SetPlayerLoc (Transformation|GetActorLocation (Variables|Player|GetPlayer))))
  (LocalVariables|SetRandomLoc (.RandomLocation (AI|Navigation|GetRandomReachablePointinRadius _output_get 4e+03 0 0)))
  (if (and (>= (Math|Vector|VectorLength (- (LocalVariables|GetPlayerLoc) (LocalVariables|GetRandomLoc))) (Variables|Player|GetMinDistanceToPlayer)) (> (Math|Vector|VectorLength (- (Variables|Wave|GetPreviousLocation) (LocalVariables|GetRandomLoc))) 5e+02))
    (Variables|Wave|SetPreviousLocation (LocalVariables|GetRandomLoc))
    (return (Math|Transform|MakeTransform (LocalVariables|GetRandomLoc)))
    (else
      (CallFunction|GetReachableTransform))))

(fn CreateChest
  (Game|SpawnActorfromClass "/Game/Blueprints/Chest/BP_Chest.BP_Chest_C" (Math|Conversions|ToTransform(Vector) (Transformation|GetActorLocation (.OutItem (Utilities|Array|Random (Variables|Chest|GetChestPossibleLocationds))))) "Undefined" "MultiplyWithRoot" 0 0)
  (Variables|Chest|SetCanCreateChest false)
  (Audio|PlaySoundatLocation "/Game/Vefects/Zap_VFX/Audio/SFX_Vefects_Zap_Big_02_Cue.SFX_Vefects_Zap_Big_02_Cue" (Transformation|GetActorLocation (Variables|Player|GetPlayer)) "0, 0, 0" 1.0 1.0 0.0 0 0 0 0)
  (return))

(fn Save
  (params (SaveGame :type Save%20Game%20Object%20Reference))
  (Variables|/Game/Blueprints/GameController/SaveGame.SaveGame_C|SetEnemyKilled SaveGame (Variables|Default|GetKilledEnemyCount))
  (bind _returnvalue (SaveGame|SaveGametoSlot SaveGame "slot1"))
  (if _returnvalue
    _))