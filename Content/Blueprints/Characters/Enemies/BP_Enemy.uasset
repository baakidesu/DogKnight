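; BP_Enemy is an enemy character that damages the player at close range and can be hurt, stunned and killed.
; PawnDetector overlaps flag the player as near, and Tick applies damage gated by a one-second cooldown.
; HitDamage lowers health and briefly flashes a hit material, while Stun temporarily zeroes walk speed and adds a Stunned tag.
; Die notifies BPGameController, which messages the spawner, then destroys the actor.
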(event OnComponentBeginOverlap(PawnDetector)
  (params (OverlappedComponent :type Primitive%20Component%20Object%20Reference) (OtherActor :type Actor%20Object%20Reference) (OtherComp :type Primitive%20Component%20Object%20Reference) (OtherBodyIndex :type Integer) (bFromSweep :type Boolean) (SweepResult :type Hit%20Result%20Structure%20%28by%20ref%29))
  (if (Actor|ActorHasTag OtherActor "Player")
    (Variables|Default|SetPawnNear true)))

(event OnComponentEndOverlap(PawnDetector)
  (params (OverlappedComponent :type Primitive%20Component%20Object%20Reference) (OtherActor :type Actor%20Object%20Reference) (OtherComp :type Primitive%20Component%20Object%20Reference) (OtherBodyIndex :type Integer))
  (if (Actor|ActorHasTag OtherActor "Player")
    (Variables|Default|SetPawnNear false)))

(event EventTick
  (params (DeltaSeconds :type Float%20%28single-precision%29))
  (if (and (Variables|Default|GetPawnNear) (Variables|Default|GetCanHit))
    (Game|Damage|ApplyDamage (Variables|Default|GetAs%20BP%20Player) 1e+01 0 0)
    (Variables|Default|SetCanHit false)
    (Utilities|FlowControl|Delay 1.0)
    (Variables|Default|SetCanHit true)))

(event EventBeginPlay
  (Variables|Default|SetInitialMaterial (Rendering|Material|GetMaterial (Variables|Character|GetMesh) 0))
  (bind _asbp_player (Utilities|Casting|CastToBP_Player (Game|Player|GetPlayerPawn 0)))
  (Variables|Default|SetAs%20BP%20Player _asbp_player)
  (Variables|Default|SetMax%20Walk%20Speed (Variables|/Script/Engine.CharacterMovementComponent|GetMaxWalkSpeed (Variables|Character|GetCharacterMovement))))

(event EventHitDamage
  (params (Damage :type Float%20%28double-precision%29))
  (bind _output_get (Variables|Default|SetHealth (- (Variables|Default|GetHealth) Damage)))
  (if (<= _output_get 0.0)
    (CallFunction|Die)
    (else
      (Rendering|Material|SetMaterial (Variables|Character|GetMesh) 0 "/Game/Materials/M_Hit.M_Hit")
      (Utilities|FlowControl|Delay 0.5)
      (Rendering|Material|SetMaterial (Variables|Character|GetMesh) 0 (Variables|Default|GetInitialMaterial)))))

(event EventStun
  (params (StunAmount :type Float%20%28double-precision%29))
  (bind _charactermovement (Variables|Character|GetCharacterMovement))
  (Variables|/Script/Engine.CharacterMovementComponent|SetMaxWalkSpeed _charactermovement 0.0)
  (Variables|Default|SetTags (Utilities|Array|MakeArray (Variables|Default|GetStunned) "Enemy"))
  (Variables|Default|SetIsStunned true)
  (Utilities|FlowControl|Delay StunAmount)
  (Variables|Default|SetTags (Utilities|Array|MakeArray "Enemy"))
  (Variables|Default|SetIsStunned false)
  (Variables|/Script/Engine.CharacterMovementComponent|SetMaxWalkSpeed _charactermovement (Variables|Default|GetMax%20Walk%20Speed))
  (Pawn|Components|CharacterMovement|SetMovementMode _charactermovement "MOVE_Walking" 0))

(fn ConstructionScript)

(fn Die
  (Rendering|Material|SetMaterial (Variables|Character|GetMesh) 0 "/Game/Materials/M_Hit.M_Hit")
  (bind _bp_gamecontroller (Variables|Default|GetBP_GameController)
    (:then
      (Default|DieMessagetoSpawner _bp_gamecontroller))
    (:else
      _))
  (Actor|DestroyActor))

(fn HitActor)