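; Throwing spell skill pickup that, once collected, periodically fires BP_Spell projectiles from the player's location.
; On overlap it removes its mesh, notifies its Chest and registers on the player, or adjusts its own Damage and destroys itself if the skill is already owned.
; A Tick-driven seconds counter triggers throws on cooldown, aimed at a random enemy with Damage and sound, or at a random yaw without either.
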(event OnComponentBeginOverlap(SM)
  (params (OverlappedComponent :type Primitive%20Component%20Object%20Reference) (OtherActor :type Actor%20Object%20Reference) (OtherComp :type Primitive%20Component%20Object%20Reference) (OtherBodyIndex :type Integer) (bFromSweep :type Boolean) (SweepResult :type Hit%20Result%20Structure%20%28by%20ref%29))
  (bind _player (Variables|Default|GetPlayer))
  (Components|DestroyComponent (Variables|Default|GetSM))
  (Utilities|FlowControl|Delay 0.0)
  (bind _chest (Variables|Default|GetChest)
    (:then
      (Default|ChestDestroy _chest self))
    (:else
      _))
  (if (Variables|/Game/Blueprints/Characters/Player/BP_Player.BP_Player_C|GetHasThrowingSpell (Variables|Default|GetPlayer))
    (Variables|Spell|SetDamage (+ (Variables|Spell|GetDamage) (Math|Float|%(Float) (Variables|Spell|GetDamage) (Variables|Spell|GetIncreaseDamagePercentage))))
    (Actor|DestroyActor)
    (else
      (Variables|System|SetCanWork true)
      (Variables|/Game/Blueprints/Characters/Player/BP_Player.BP_Player_C|SetHasThrowingSpell _player true)
      (Variables|/Game/Blueprints/Characters/Player/BP_Player.BP_Player_C|SetThrowingSpell _player self))))

(event EventTick
  (params (DeltaSeconds :type Float%20%28single-precision%29))
  (CallFunction|CountSeconds DeltaSeconds)
  (if (and (>= (Variables|System|GetCurrentTime) (Variables|Spell|GetSpellCooldown)) (Variables|System|GetCanWork))
    (Variables|System|SetCurrentTime 0)
    (CallFunction|ThrowSpell)))

(event EventBeginPlay
  (bind _asbp_player (Utilities|Casting|CastToBP_Player (Game|Player|GetPlayerPawn 0)))
  (Variables|Default|SetPlayer _asbp_player))

(fn ConstructionScript)

(fn CountSeconds
  (params (Delta%20Time :type Float%20%28double-precision%29))
  (bind _output_get (Variables|System|SetAccumulatedTime (+ Delta%20Time (Variables|System|GetAccumulatedTime))))
  (if (>= _output_get 1.0)
    (Variables|System|SetAccumulatedTime (- (Variables|System|GetAccumulatedTime) 1.0))
    (if (Variables|System|GetCanWork)
      (Math|Integer|IncrementInt (Variables|System|GetCurrentTime)
        (:%20%20
          _))
      (else
        (Variables|System|SetCurrentTime 0)))
    (return)))

(fn ThrowSpell
  (bind _returnvalue (CallFunction|GetPlayerLocation))
  (bind _output_get (LocalVariables|SetTarget (.OutItem (Utilities|Array|Random (Variables|/Game/Blueprints/Characters/Player/BP_Player.BP_Player_C|GetEnemies (Variables|Default|GetPlayer))))))
  (Utilities|IsValid _output_get
    (:Is%20Valid
      (bind _returnvalue_2 (Game|SpawnActorfromClass "/Game/Blueprints/AdditionalSkills/ThrowingSpell/BP_Spell.BP_Spell_C" (Math|Transform|MakeTransform _returnvalue (Math|Rotator|FindLookatRotation _returnvalue (Transformation|GetActorLocation (LocalVariables|GetTarget))) "1.000000,1.000000,1.000000") "Undefined" "MultiplyWithRoot" 0 0))
      (Audio|PlaySound2D "/Game/Sounds/S_Spell.S_Spell" 1.0 1.0 0.0 0 0)
      (Variables|/Game/Blueprints/AdditionalSkills/ThrowingSpell/BP_Spell.BP_Spell_C|SetDamage _returnvalue_2 (Variables|Spell|GetDamage)))
    (:Is%20Not%20Valid
      (Game|SpawnActorfromClass "/Game/Blueprints/AdditionalSkills/ThrowingSpell/BP_Spell.BP_Spell_C" (Math|Transform|MakeTransform (CallFunction|GetPlayerLocation) (Math|Rotator|MakeRotator 0.0 0.0 (Math|Random|RandomFloatinRange 0.0 3.6e+02)) "1.000000,1.000000,1.000000") "Undefined" "MultiplyWithRoot" 0 0))))

(fn GetPlayerLocation
  (bind _player (Variables|Default|GetPlayer))
  (bind _returnvalue (Transformation|GetActorLocation _player))
  (return (Math|Vector|MakeVector (.x _returnvalue) (.y _returnvalue) (.z _returnvalue))))